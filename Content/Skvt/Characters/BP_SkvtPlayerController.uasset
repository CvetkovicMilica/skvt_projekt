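; Player controller for Skvt that lets the player cycle control between the BP_SkvtBaseChar characters in the level.
; On BeginPlay it adds the default, pawn swap and camera Enhanced Input mapping contexts.
; The swap input gathers every base character, finds the current pawn in that list and possesses the next one, wrapping to the first after the last.
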(event `self.ReceiveBeginPlay`
  (bind _returnvalue (pcsubsystem `EnhancedInputLocalPlayerSubsystem` self))
  (`/Engine/EditorBlueprintResources/StandardMacros.IsValid` _returnvalue
    (:`Is Valid`
      (`EnhancedInputSubsystemInterface.AddMappingContext` _returnvalue "/Game/ThirdPerson/Input/IMC_Default.IMC_Default" 0 (struct))
      (`EnhancedInputSubsystemInterface.AddMappingContext` _returnvalue "/Game/Skvt/Characters/Input/IMC_SwapPawn.IMC_SwapPawn" 0 (struct))
      (`EnhancedInputSubsystemInterface.AddMappingContext` _returnvalue "/Game/Skvt/Characters/Input/IMC_Camera.IMC_Camera" 0 (struct)))))

(event `EnhancedInput|/Game/Skvt/Characters/Input/Actions/IA_Swap`
  (params (ActionValue :type Boolean) (ElapsedSeconds :type "Float (double-precision)") (TriggeredSeconds :type "Float (double-precision)") (InputAction :type "InputAction Object Reference" :default "/Game/Skvt/Characters/Input/Actions/IA_Swap.IA_Swap"))
  (:`Triggered`
    (bind _outactors (`GameplayStatics.GetAllActorsOfClass` "/Game/Skvt/Characters/BP_SkvtBaseChar.BP_SkvtBaseChar_C"))
    (bind _asbp_skvt_base_char (cast `/Game/Skvt/Characters/BP_SkvtBaseChar` (`self.K2_GetPawn`)))
    (bind _returnvalue (`KismetArrayLibrary.Array_Find` _outactors _asbp_skvt_base_char))
    (if (>= _returnvalue 0)
      (bind _returnvalue_2 (+ _returnvalue 1))
      (if (== _returnvalue_2 (`KismetArrayLibrary.Array_Length` _outactors))
        (`self.Possess` (`|GetArrayItem` _outactors))
        (else
          (`self.Possess` (`|GetArrayItem` _outactors _returnvalue_2)))))))

(fn `UserConstructionScript`)